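; Per-player pawn for a frog-feeding minigame, where the player catapults randomly sized peas at a team-colored frog.
; Button, flex or trigger inputs pick one of three launch strengths, which must match the pea's size to land.
; Timelines animate the drop, throw arc and frog growth.
; A hit plays the eating montage, whose "Ate" notify scores a point and respawns the pea, while misses just respawn it.
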(event Custom|AddPea
  (bind _pea (Variables|Default|GetPea))
  ;[1 1 1] Adds back a Pea
  (Transformation|AttachComponentToComponent (Variables|Default|GetPea) (Variables|Default|GetPeaLocation) "None" "SnapToTarget" "SnapToTarget" "SnapToTarget" true)
  (bind _output_get (Variables|Default|SetSize (Math|Random|RandomInteger 3)))
  (Rendering|Material|SetScalarParameterValueonMaterials (Variables|Default|GetPea) "Index" (Math|Conversions|ToFloat(Integer) (Variables|Default|GetSize)))
  (Transformation|SetRelativeScale3D (Variables|Default|GetPea) (Math|Conversions|ToVector(Float) (Utilities|Select :Index _output_get :Option%200 0.5 :Option%201 0.75 :Option%202 1.0)))
  (bind _zval (Timeline|FallingPea PlayFromStart)
    (:Update
      (Transformation|SetRelativeLocation _pea (Math|Vector|MakeVector 0.0 0.0 (Math|Float|Lerp 1e+03 0.0 _zval)) false false))
    (:Finished
      (Variables|Default|SetPeaReady true)
      (Transformation|SetRelativeLocation _pea (Math|Vector|MakeVector 0.0 0.0 0.0) false false))))

(event Custom|Montage
  (params (StartingSection :type Name :default "start") (Feed :type Boolean))
  ;[1 1 1] Munching and wobbling and such
  (bind _notifyname (Animation|Montage|PlayMontage (Variables|Default|Getfrog) (Variables|Default|GetMontage%20to%20Play) 1.0 0.0 StartingSection)
    (:then
      (if Feed
        (bind _output_get (Variables|Default|SetRelative%20Scale%203D (Variables|/Script/Engine.SceneComponent|GetRelativeScale3D (Variables|Default|Getfrog))))
        (bind _newtrack_0 (Timeline|GrowFrog PlayFromStart)
          (:Update
            (Transformation|SetRelativeScale3D (Variables|Default|Getfrog) (Math|Vector|Lerp(Vector) _output_get (+ _output_get 0.1) _newtrack_0))))))
    (:OnNotifyBegin
      (if (== _notifyname "Ate")
        (CallFunction|AddPea)
        (Class|BasePointCounter|AddPoints (Class|MinigameBase|GetPointCounter (Variables|Default|GetMinigame)) (Variables|Default|GetPlayerNumber) 1)))))

(event Custom|Launch
  (params (Strength :type Integer))
  (bind _frog (Variables|Default|Getfrog))
  ;[1 1 1] Launch Pea
  (if (Variables|Default|GetPeaReady)
    (Variables|Default|SetAddedForce (- Strength (Variables|Default|GetSize)))
    (Variables|Default|SetPeaReleased false)
    (Variables|Default|SetPeaReady false)
    (bind (_direction _zarc _wood _yark) (Timeline|ThrowPea PlayFromStart)
      (:Update
        (Transformation|SetRelativeRotation (Variables|Default|Getwood_Cube) (Math|Rotator|Lerp(Rotator) "0, 0, 0" "-40.000000,0.000000,0.000000" _wood true) false false)
        (if (Variables|Default|GetPeaReleased)
          (Transformation|SetRelativeLocation (Variables|Default|GetPea) (Math|Vector|MakeVector (.x (Math|Vector|Lerp(Vector) (Variables|Default|GetPeaOG) (+ (Variables|/Script/Engine.SceneComponent|GetRelativeLocation _frog) (* (Variables|/Script/Engine.SceneComponent|GetRelativeScale3D _frog) "0.000000,80.000000,100.000000") (Math|Vector|MakeVector 0.0 (* (Variables|Default|GetAddedForce) -3e+02) 0.0)) _yark)) (.y (Math|Vector|Lerp(Vector) (Variables|Default|GetPeaOG) (+ (Variables|/Script/Engine.SceneComponent|GetRelativeLocation _frog) (* (Variables|/Script/Engine.SceneComponent|GetRelativeScale3D _frog) "0.000000,80.000000,100.000000") (Math|Vector|MakeVector 0.0 (* (Variables|Default|GetAddedForce) -3e+02) 0.0)) _yark)) (+ (.z (Math|Vector|Lerp(Vector) (Variables|Default|GetPeaOG) (+ (Variables|/Script/Engine.SceneComponent|GetRelativeLocation _frog) (* (Variables|/Script/Engine.SceneComponent|GetRelativeScale3D _frog) "0.000000,80.000000,100.000000") (Math|Vector|MakeVector 0.0 (* (Variables|Default|GetAddedForce) -3e+02) 0.0)) _yark)) (* _zarc 3e+02))) false false)))
      (:Finished
        (if (== (Variables|Default|GetAddedForce) 0)
          (CallFunction|Montage "GetFood" true)
          (else
            (CallFunction|AddPea))))
      (:RelesePea
        (Variables|Default|SetPeaReleased true)
        (Transformation|AttachComponentToComponent (Variables|Default|GetPea) (Variables|Default|GetDefaultSceneRoot) "None" "KeepRelative" "KeepRelative" "KeepRelative" true)
        (Variables|Default|SetPeaOG (Variables|/Script/Engine.SceneComponent|GetRelativeLocation (Variables|Default|GetPea)))))))

(event Input|EnhancedActionEvents|EnhancedInputActionIA_LeftTrigger
  (params (ActionValue :type Float%20%28double-precision%29) (ElapsedSeconds :type Float%20%28double-precision%29) (TriggeredSeconds :type Float%20%28double-precision%29) (InputAction :type Input%20Action%20Object%20Reference :default "/MinigameCore/Input/IA_LeftTrigger.IA_LeftTrigger"))
  (:Started
    (Utilities|FlowControl|Delay 0.1)
    (if (> ActionValue 0.05)
      (CallFunction|Launch (Math|Integer|SelectInt 0 (Math|Integer|SelectInt 1 2 (Math|Float|InRange(Float) ActionValue 0.4 0.7)) (Math|Float|InRange(Float) ActionValue 0.05 0.4))))))

(event Input|EnhancedActionEvents|EnhancedInputActionIA_StrongFlex
  (params (ActionValue :type Boolean) (ElapsedSeconds :type Float%20%28double-precision%29) (TriggeredSeconds :type Float%20%28double-precision%29) (InputAction :type Input%20Action%20Object%20Reference :default "/LimbitlessBluetoothPlugin/InputActions/IA_StrongFlex.IA_StrongFlex"))
  (:Started
    (CallFunction|Launch 2)))

(event Input|EnhancedActionEvents|EnhancedInputActionIA_Button1
  (params (ActionValue :type Boolean) (ElapsedSeconds :type Float%20%28double-precision%29) (TriggeredSeconds :type Float%20%28double-precision%29) (InputAction :type Input%20Action%20Object%20Reference :default "/MinigameCore/Input/IA_Button1.IA_Button1"))
  (CallFunction|Launch))

(event Input|EnhancedActionEvents|EnhancedInputActionIA_MediumFlex
  (params (ActionValue :type Boolean) (ElapsedSeconds :type Float%20%28double-precision%29) (TriggeredSeconds :type Float%20%28double-precision%29) (InputAction :type Input%20Action%20Object%20Reference :default "/LimbitlessBluetoothPlugin/InputActions/IA_MediumFlex.IA_MediumFlex"))
  (:Started
    (CallFunction|Launch 1)))

(event Input|EnhancedActionEvents|EnhancedInputActionIA_LightFlex
  (params (ActionValue :type Boolean) (ElapsedSeconds :type Float%20%28double-precision%29) (TriggeredSeconds :type Float%20%28double-precision%29) (InputAction :type Input%20Action%20Object%20Reference :default "/LimbitlessBluetoothPlugin/InputActions/IA_LightFlex.IA_LightFlex"))
  (:Started
    (CallFunction|Launch)))

(event EventBeginPlay
  ;[0.2044 1 0.1041] Begin Play
  (CallFunction|AddPea)
  (CallFunction|SetFrogMaterial)
  (Utilities|FlowControl|Delay (Utilities|Select :Index (Variables|Default|GetPlayerNumber) :Option%200 0.1 :Option%201 0.2 :Option%202 0.3 :Option%203 0.4))
  (CallFunction|Montage "start" false))

(event Input|KeyboardEvents|F
  (params (Key :type Key%20Structure :default "None"))
  (:Pressed
    (CallFunction|Launch 1)))

(event Input|KeyboardEvents|E
  (params (Key :type Key%20Structure :default "None"))
  (:Pressed
    (CallFunction|Launch 2)))

(event Input|KeyboardEvents|G
  (params (Key :type Key%20Structure :default "None"))
  (:Pressed
    (for _index (range 0 3)
      (Class|MinigameBase|ReadyPlayer (Variables|Default|GetMinigame) _index false))))

(fn ConstructionScript)

(fn SetFrogMaterial
  (Rendering|Material|SetMaterial (Variables|Default|Getfrog) 2 (Utilities|Select :Index (Variables|Default|GetPlayerNumber) :Option%200 "/Game/Imports/frog/MI_FrogYellow.MI_FrogYellow" :Option%201 "/Game/Imports/frog/MI_FrogRed.MI_FrogRed" :Option%202 "/Game/Imports/frog/M_FrogGreen.M_FrogGreen" :Option%203 "/Game/Imports/frog/MI_FrogPurple.MI_FrogPurple")))